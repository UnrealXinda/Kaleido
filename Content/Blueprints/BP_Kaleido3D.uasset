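; BP_Kaleido3D is an actor that fills a 3D grid with copies of the KaleidoInstancedMesh instanced mesh.
; The construction script builds it with three nested DoN nodes used as loops, re-entered and reset to step through SizeX, SizeY and SizeZ.
; Each counter times DistanceX, DistanceY or DistanceZ sets an instance's position, with no rotation and unit scale.
; The event graph holds no active logic.
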(fn `UserConstructionScript`
  (bind _counter (`/Engine/EditorBlueprintResources/StandardMacros.Do N` (`self.SizeZ`) :!label _label)
    (:`Exit`
      (`|ExecutionSequence`
        (:`then_0`
          (bind _counter_2 (`/Engine/EditorBlueprintResources/StandardMacros.Do N` (`self.SizeY`) :!label _label_2)
            (:`Exit`
              (`|ExecutionSequence`
                (:`then_0`
                  (bind _counter_3 (`/Engine/EditorBlueprintResources/StandardMacros.Do N` (`self.SizeX`) :!label _label_3)
                    (:`Exit`
                      (`|ExecutionSequence`
                        (:`then_0`
                          (`InstancedStaticMeshComponent.AddInstance` (`self.KaleidoInstancedMesh`) (`KismetMathLibrary.MakeTransform` (`KismetMathLibrary.MakeVector` (* _counter_3 (`self.DistanceX`)) (* _counter_2 (`self.DistanceY`)) (* _counter (`self.DistanceZ`))))))
                        (:`then_1`
                          (goto _label_3))))))
                (:`then_1`
                  (goto _label_3 :!via `Reset`))
                (:`then_2`
                  (goto _label_2))))))
        (:`then_1`
          (goto _label_2 :!via `Reset`))
        (:`then_2`
          (goto _label))))))